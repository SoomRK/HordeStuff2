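; Server-side bank for Mordhau Horde that lets players deposit and withdraw coins through chat commands, keeping balances across matches.
; Config sets name, fee, limits and disabled maps; game-mode login and chat hooks drive account creation and teller broadcasts.
; Accounts are "PlayFabID=balance,withdrawalLeft" strings, loaded from PointBank.txt with allowances reset and saved when Tick detects match end.
; Coin cheats by non-super admins shut the bank for the match.
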(event Custom|CustomEvent_0
  (params (Sender :type Actor%20Object%20Reference) (Msg :type String) (Type :type Name))
  (bind (_returnvalue _returnvalue1) (CallFunction|MessageHasCommand Msg "!deposit"))
  (bind (_returnvalue_2 _returnvalue1_2) (CallFunction|MessageHasCommand Msg "!withdraw"))
  (bind _bankname (Variables|Default|GetBankName))
  (bind _bankname_2 (Variables|Default|GetBankName))
  (bind _bankname_3 (Variables|Default|GetBankName))
  (bind _bankname_4 (Variables|Default|GetBankName))
  (bind _account_limit (Variables|Default|GetAccount%20Limit))
  (bind _bankname_5 (Variables|Default|GetBankName))
  (if (not (Variables|Default|GetPreventRec))
    (Development|PrintString "OnMessageBroadcasted_Event")
    (bind _asbp_horde_player_controller (Utilities|Casting|CastToBP_HordePlayerController Sender))
    (bind _output_get (Variables|Default|SetAs%20BP%20Horde%20Player%20Controller _asbp_horde_player_controller))
    (Variables|Default|SetPreventRec true)
    (Variables|Default|SetNewVar_0 0)
    (Utilities|FlowControl|Sequence
      (:then_0
        (if (not (CallFunction|IsSuperAdmin _output_get))
          (if (Class|MordhauPlayerController|IsAdmin _output_get)
            (if (or (.ReturnValue (CallFunction|MessageHasCommand Msg ".coinsall")) (.ReturnValue (CallFunction|MessageHasCommand Msg ".coins")))
              (Variables|Default|SetIsDisabled true)
              (Utilities|BroadcastMacro
                (:Completed
                  (CallFunction|Broadcast (Utilities|String|Append _bankname " has detected Admin Stimulus, to prevent Inflation, " _bankname " has shut down for the remainder of the match. No deposits or withdrawl's can be made."))))))))
      (:then_1
        (if _returnvalue
          (bind _output_get_2 (Variables|Default|SetNewVar_0 (Math|Conversions|ToInteger(Byte) _returnvalue1)))
          (if (> _output_get_2 0)
            (bind _isdisabled (CallFunction|NotifyDisabled))
            (if (not _isdisabled)
              (bind _asbp_horde_player_state (Utilities|Casting|CastToBP_HordePlayerState (Variables|/Script/Engine.Controller|GetPlayerState _output_get)))
              (if (>= (Variables|/Game/Mordhau/Blueprints/GameModes/Horde/BP_HordePlayerState.BP_HordePlayerState_C|GetCoins _asbp_horde_player_state) _output_get_2)
                (Utilities|BroadcastMacro
                  (:Completed
                    (CallFunction|Broadcast (Utilities|String|Append (PlayerState|GetPlayerName _asbp_horde_player_state) " has attempted to deposit :: " (Utilities|String|ToString(Integer) _output_get_2) " :: Coins to " _bankname_3))
                    (bind (_returnvalue_3 _array_index) (CallFunction|PrepareEntry _output_get))
                    (if _returnvalue_3
                      (if (> (+ _output_get_2 (CallFunction|GetEntryBalance _array_index)) _account_limit)
                        (Utilities|BroadcastMacro
                          (:Completed
                            (CallFunction|Broadcast (Utilities|String|Append _bankname_4 " Teller: Sorry " (PlayerState|GetPlayerName _asbp_horde_player_state) ", this would put you over the max allowed amount for your account. Your Max allowed amount is currently :: " (Utilities|String|ToString(Integer) _account_limit) " ::"))))
                        (else
                          (Utilities|BroadcastMacro
                            (:Completed
                              (CallFunction|Broadcast (Utilities|String|Append _bankname_4 " Teller: Your account balance has been updated, your new current amount is :: " (Utilities|String|ToString(Integer) (+ _output_get_2 (CallFunction|GetEntryBalance _array_index))) " :: Thank you for being a valued customer of " _bankname_4 (Utilities|Select :Index (Math|Random|RandomIntegerinRange 0 5) :Option%200 (Utilities|String|Append ". Slay them all " (PlayerState|GetPlayerName _asbp_horde_player_state) "!") :Option%201 ". Enjoy the Match!" :Option%202 ". I am humbled by your skills, sir!" :Option%203 ". Your form, and execution, are exquisite!" :Option%204 ". It is an honor to meet such a fine combatant!" :Option%205 ". You have the heart of a lion!")))
                              (CallFunction|SetEntryBalance _array_index (+ _output_get_2 (CallFunction|GetEntryBalance _array_index)))
                              (Variables|/Game/Mordhau/Blueprints/GameModes/Horde/BP_HordePlayerState.BP_HordePlayerState_C|SetCoins _asbp_horde_player_state (- (Variables|/Game/Mordhau/Blueprints/GameModes/Horde/BP_HordePlayerState.BP_HordePlayerState_C|GetCoins _asbp_horde_player_state) _output_get_2))))))
                      (else
                        (Utilities|BroadcastMacro
                          (:Completed
                            (CallFunction|Broadcast (Utilities|String|Append "ERROR: " "ArrayIndex==" (Utilities|String|ToString(Integer) _array_index) "EntryAmmount==" (Utilities|String|ToString(Integer) (CallFunction|GetEntryBalance _array_index))))))))))
                (else
                  (Utilities|BroadcastMacro
                    (:Completed
                      (CallFunction|Broadcast (Utilities|String|Append _bankname_3 " Teller: " (PlayerState|GetPlayerName _asbp_horde_player_state) ", you do not have enough coins to make this Deposit."))))))))
          (elif _returnvalue_2
            (bind _isdisabled_2 (CallFunction|NotifyDisabled))
            (if (not _isdisabled_2)
              (bind (_returnvalue_4 _array_index_2) (CallFunction|PrepareEntry _output_get))
              (if _returnvalue_4
                (bind _output_get_3 (Variables|Default|SetNewVar_0 (Math|Conversions|ToInteger(Byte) _returnvalue1_2)))
                (if (and (> _output_get_3 0) (not (> _output_get_3 (CallFunction|GetAmountLeft _array_index_2))))
                  (bind _asbp_horde_player_state_2 (Utilities|Casting|CastToBP_HordePlayerState (Variables|/Script/Engine.Controller|GetPlayerState _output_get)))
                  (Utilities|BroadcastMacro
                    (:Completed
                      (CallFunction|Broadcast (Utilities|String|Append (PlayerState|GetPlayerName _asbp_horde_player_state_2) " has attempted to withdraw :: " (Utilities|String|ToString(Integer) _output_get_3) " :: Coins from " _bankname_5 ". With a Fee of :: " (Utilities|String|ToString(Integer) (Math|Float|Truncate (* _output_get_3 (Variables|Default|GetFee)))) " ::"))
                      (if (>= (CallFunction|GetEntryBalance _array_index_2) (+ _output_get_3 (Math|Float|Truncate (* _output_get_3 (Variables|Default|GetFee)))))
                        (Utilities|BroadcastMacro
                          (:Completed
                            (CallFunction|Broadcast (Utilities|String|Append _bankname_2 "Teller: Your withdrawl is accepted. Your account balance has been updated, new current balance is :: " (Utilities|String|ToString(Integer) (- (CallFunction|GetEntryBalance _array_index_2) (+ _output_get_3 (Math|Float|Truncate (* _output_get_3 (Variables|Default|GetFee)))))) " :: Thank you for being a valued customer of " _bankname_2 (Utilities|Select :Index (Math|Random|RandomIntegerinRange 0 5) :Option%200 (Utilities|String|Append ". Slay them all " (PlayerState|GetPlayerName _asbp_horde_player_state) "!") :Option%201 ". Enjoy the Match!" :Option%202 ". I am humbled by your skills, sir!" :Option%203 ". Your form, and execution, are exquisite!" :Option%204 ". It is an honor to meet such a fine combatant!" :Option%205 ". You have the heart of a lion!") " 
There is currently :: " (Utilities|String|ToString(Integer) (- (CallFunction|GetAmountLeft _array_index_2) _output_get_3)) " :: Remaining available withdrawl for this match."))
                            (CallFunction|SetEntryBalance _array_index_2 (- (CallFunction|GetEntryBalance _array_index_2) (+ _output_get_3 (Math|Float|Truncate (* _output_get_3 (Variables|Default|GetFee))))))
                            (CallFunction|SetAmountLeft _array_index_2 (- (CallFunction|GetAmountLeft _array_index_2) _output_get_3))
                            (Variables|/Game/Mordhau/Blueprints/GameModes/Horde/BP_HordePlayerState.BP_HordePlayerState_C|SetCoins _asbp_horde_player_state_2 (+ (Variables|/Game/Mordhau/Blueprints/GameModes/Horde/BP_HordePlayerState.BP_HordePlayerState_C|GetCoins _asbp_horde_player_state_2) _output_get_3))))
                        (else
                          (Utilities|BroadcastMacro
                            (:Completed
                              (CallFunction|Broadcast (Utilities|String|Append _bankname_5 " Teller: Sorry " (PlayerState|GetPlayerName _asbp_horde_player_state_2) ", You do not have enough coins in your account to make this Transaction. "))))))))
                  (else
                    (Utilities|BroadcastMacro
                      (:Completed
                        (CallFunction|Broadcast (Utilities|String|Append (Variables|Default|GetBankName) " Teller: Sorry, this amount would put you over your withdraw limit for the match."))))))))
            (elif (.ReturnValue (CallFunction|MessageHasCommand Msg "!bankhelp"))
              (Variables|Default|SetNewVar_1 "")
              (bind _isdisabled_3 (CallFunction|NotifyDisabled))
              (bind _array_index_3 (CallFunction|PrepareEntry _output_get))
              (Variables|Default|SetNewVar_1 (Utilities|String|Append "Help Menu 
" "!deposit amount       
 // Deposits the specified amount, assuming you have it. 
!withdraw amount  
// Will withdraw from bank account if you have the funds/the bank has the funds. 
 
Current Account Balance :: " (Utilities|String|ToString(Integer) (CallFunction|GetEntryBalance _array_index_3)) " :: 
Bank Status :: " (Utilities|String|SelectString "DISABLED" "ENABLED" _isdisabled_3) " :: 
Remaining available withdrawl for the match :: " (Utilities|String|ToString(Integer) (CallFunction|GetAmountLeft _array_index_3)) " ::"))
              (Utilities|BroadcastMacro
                (:Completed
                  (CallFunction|Broadcast (Utilities|String|Append "Help Menu 
" "!deposit amount       
 // Deposits the specified amount, assuming you have it. 
!withdraw amount  
// Will withdraw from bank account if you have the funds/the bank has the funds. 
 
Current Account Balance :: " (Utilities|String|ToString(Integer) (CallFunction|GetEntryBalance _array_index_3)) " :: 
Bank Status :: " (Utilities|String|SelectString "DISABLED" "ENABLED" _isdisabled_3) " :: 
Remaining available withdrawl for the match :: " (Utilities|String|ToString(Integer) (CallFunction|GetAmountLeft _array_index_3)) " ::"))))))))
      (:then_2
        (Variables|Default|SetPreventRec false)))))

(event Custom|Event_ChatCommand
  (params (NewParam :type BP%20Horde%20Player%20Controller%20Object%20Reference) (NewParam2 :type String) (NewParam3 :type Integer) (NewParam4 :type String))
  (bind _amount (CallFunction|GetEntryBalance NewParam3))
  (bind _returnvalue (CallFunction|GetAmountLeft NewParam3))
  (bind _bankname (Variables|Default|GetBankName))
  (bind _account_limit (Variables|Default|GetAccount%20Limit))
  (bind _bankname_2 (Variables|Default|GetBankName))
  (bind _bankname_3 (Variables|Default|GetBankName))
  (bind _bankname_4 (Variables|Default|GetBankName))
  (bind _bankname_5 (Variables|Default|GetBankName))
  (switch string NewParam2
    (:!bankhelp
      (Variables|Default|SetNewVar_1 "")
      (bind _isdisabled (CallFunction|NotifyDisabled))
      (Variables|Default|SetNewVar_1 (Utilities|String|Append "Help Menu 
" "!deposit amount       
 // Deposits the specified amount, assuming you have it. 
!withdraw amount  
// Will withdraw from bank account if you have the funds/the bank has the funds. 
 
Current Account Balance :: " (Utilities|String|ToString(Integer) (CallFunction|GetEntryBalance NewParam3)) " :: 
Bank Status :: " (Utilities|String|SelectString "DISABLED" "ENABLED" _isdisabled) " :: 
Remaining available withdrawl for the match :: " (Utilities|String|ToString(Integer) (CallFunction|GetAmountLeft NewParam3)) " ::"))
      (Utilities|BroadcastMacro
        (:Completed
          (CallFunction|Broadcast (Utilities|String|Append "Help Menu 
" "!deposit amount       
 // Deposits the specified amount, assuming you have it. 
!withdraw amount  
// Will withdraw from bank account if you have the funds/the bank has the funds. 
 
Current Account Balance :: " (Utilities|String|ToString(Integer) (CallFunction|GetEntryBalance NewParam3)) " :: 
Bank Status :: " (Utilities|String|SelectString "DISABLED" "ENABLED" _isdisabled) " :: 
Remaining available withdrawl for the match :: " (Utilities|String|ToString(Integer) (CallFunction|GetAmountLeft NewParam3)) " ::")))))
    (:!deposit
      (bind _output_get (Variables|Default|SetNewVar_0 (Math|Conversions|ToInteger(Byte) NewParam4)))
      (if (> _output_get 0)
        (bind _asbp_horde_player_state (Utilities|Casting|CastToBP_HordePlayerState (Variables|/Script/Engine.Controller|GetPlayerState NewParam)))
        (if (>= (Variables|/Game/Mordhau/Blueprints/GameModes/Horde/BP_HordePlayerState.BP_HordePlayerState_C|GetCoins _asbp_horde_player_state) _output_get)
          (Utilities|BroadcastMacro
            (:Completed
              (CallFunction|Broadcast (Utilities|String|Append (PlayerState|GetPlayerName _asbp_horde_player_state) " has attempted to deposit :: " (Utilities|String|ToString(Integer) _output_get) " :: Coins to " _bankname_3))
              (if (> (+ _output_get (CallFunction|GetEntryBalance NewParam3)) _account_limit)
                (Utilities|BroadcastMacro
                  (:Completed
                    (CallFunction|Broadcast (Utilities|String|Append _bankname_2 " Teller: Sorry " (PlayerState|GetPlayerName _asbp_horde_player_state) ", this would put you over the max allowed amount for your account. Your Max allowed amount is currently :: " (Utilities|String|ToString(Integer) _account_limit) " ::"))))
                (else
                  (Utilities|BroadcastMacro
                    (:Completed
                      (CallFunction|Broadcast (Utilities|String|Append _bankname_2 " Teller: Your account balance has been updated, your new current amount is :: " (Utilities|String|ToString(Integer) (+ _output_get (CallFunction|GetEntryBalance NewParam3))) " :: Thank you for being a valued customer of " _bankname_2 (Utilities|Select :Index (Math|Random|RandomIntegerinRange 0 5) :Option%200 (Utilities|String|Append ". Slay them all " (PlayerState|GetPlayerName _asbp_horde_player_state) "!") :Option%201 ". Enjoy the Match!" :Option%202 ". I am humbled by your skills, sir!" :Option%203 ". Your form, and execution, are exquisite!" :Option%204 ". It is an honor to meet such a fine combatant!" :Option%205 ". You have the heart of a lion!")))
                      (CallFunction|SetEntryBalance NewParam3 (+ _output_get (CallFunction|GetEntryBalance NewParam3)))
                      (Variables|/Game/Mordhau/Blueprints/GameModes/Horde/BP_HordePlayerState.BP_HordePlayerState_C|SetCoins _asbp_horde_player_state (- (Variables|/Game/Mordhau/Blueprints/GameModes/Horde/BP_HordePlayerState.BP_HordePlayerState_C|GetCoins _asbp_horde_player_state) _output_get))))))))
          (else
            (Utilities|BroadcastMacro
              (:Completed
                (CallFunction|Broadcast (Utilities|String|Append _bankname_3 " Teller: " (PlayerState|GetPlayerName _asbp_horde_player_state) ", you do not have enough coins to make this Deposit."))))))))
    (:!withdraw
      (bind _output_get_2 (Variables|Default|SetNewVar_0 (Math|Conversions|ToInteger(Byte) NewParam4)))
      (if (and (> _output_get_2 0) (not (> _output_get_2 _returnvalue)))
        (bind _asbp_horde_player_state_2 (Utilities|Casting|CastToBP_HordePlayerState (Variables|/Script/Engine.Controller|GetPlayerState NewParam)))
        (Utilities|BroadcastMacro
          (:Completed
            (CallFunction|Broadcast (Utilities|String|Append (PlayerState|GetPlayerName _asbp_horde_player_state_2) " has attempted to withdraw :: " (Utilities|String|ToString(Integer) _output_get_2) " :: Coins from " _bankname ". With a Fee of :: " (Utilities|String|ToString(Integer) (Math|Float|Truncate (* _output_get_2 (Variables|Default|GetFee)))) " ::"))
            (if (>= _amount (+ _output_get_2 (Math|Float|Truncate (* _output_get_2 (Variables|Default|GetFee)))))
              (Utilities|BroadcastMacro
                (:Completed
                  (CallFunction|Broadcast (Utilities|String|Append _bankname_4 "Teller: Your withdrawl is accepted. Your account balance has been updated, new current balance is :: " (Utilities|String|ToString(Integer) (- _amount (+ _output_get_2 (Math|Float|Truncate (* _output_get_2 (Variables|Default|GetFee)))))) " :: Thank you for being a valued customer of " _bankname_4 "" " 
There is currently :: " (Utilities|String|ToString(Integer) (- _returnvalue _output_get_2)) " :: Remaining available withdrawl for this match."))
                  (CallFunction|SetAmountLeft NewParam3 (- _returnvalue _output_get_2))
                  (CallFunction|SetEntryBalance NewParam3 (- _amount (+ _output_get_2 (Math|Float|Truncate (* _output_get_2 (Variables|Default|GetFee))))))
                  (Variables|/Game/Mordhau/Blueprints/GameModes/Horde/BP_HordePlayerState.BP_HordePlayerState_C|SetCoins _asbp_horde_player_state_2 (+ (Variables|/Game/Mordhau/Blueprints/GameModes/Horde/BP_HordePlayerState.BP_HordePlayerState_C|GetCoins _asbp_horde_player_state_2) _output_get_2))))
              (else
                (Utilities|BroadcastMacro
                  (:Completed
                    (CallFunction|Broadcast (Utilities|String|Append _bankname " Teller: Sorry " (PlayerState|GetPlayerName _asbp_horde_player_state_2) ", You do not have enough coins in your account to make this Transaction. "))))))))
        (else
          (Utilities|BroadcastMacro
            (:Completed
              (CallFunction|Broadcast (Utilities|String|Append (Variables|Default|GetBankName) " Teller: Sorry, this amount would put you over your withdraw limit for the match.")))))))
    (:.coins
      (if (not (CallFunction|IsSuperAdmin NewParam)) :!label _label
        (if (Class|MordhauPlayerController|IsAdmin NewParam)
          (Variables|Default|SetIsDisabled true)
          (Utilities|BroadcastMacro
            (:Completed
              (CallFunction|Broadcast (Utilities|String|Append _bankname_5 " has detected Admin Stimulus, to prevent Inflation, " _bankname_5 " has shut down for the remainder of the match. No deposits or withdrawl's can be made.")))))))
    (:.coinsall
      (goto _label))))

(event Custom|CustomEvent_1
  (params (NewPlayer :type Player%20Controller%20Object%20Reference))
  (bind _bankname (Variables|Default|GetBankName))
  (bind _maxwithdraw (Variables|Default|GetMaxWithdraw))
  (bind _isdisabled (Variables|Default|GetIsDisabled))
  (bind _returnvalue (Utilities|String|SelectString "DISABLED" "ENABLED" _isdisabled))
  (Utilities|FlowControl|Delay 1.0)
  (Development|PrintString "OnAfterLogin_Event")
  (bind _asbp_horde_player_controller (Utilities|Casting|CastToBP_HordePlayerController NewPlayer))
  (bind (_returnvalue_2 _array_index) (CallFunction|PrepareEntry _asbp_horde_player_controller))
  (if _returnvalue_2
    (Utilities|BroadcastMacro
      (:Completed
        (CallFunction|Broadcast (Utilities|String|Append _bankname " is " _returnvalue ". " (PlayerState|GetPlayerName (Variables|/Script/Engine.Controller|GetPlayerState _asbp_horde_player_controller)) ", your account has been found in our database, your current balance is :: " (Utilities|String|ToString(Integer) (CallFunction|GetEntryBalance _array_index)) " :: Type !bankhelp in chat for a list of commands!" " 
Your maximum allowed withdrawl for the match is  :: " (Utilities|String|ToString(Integer) _maxwithdraw) " ::"))))
    (else
      (Utilities|BroadcastMacro
        (:Completed
          (CallFunction|Broadcast (Utilities|String|Append _bankname " is " _returnvalue ". Welcome New Customer! You do not currently have a bank account made, a new one has been setup for you. The terms of your agreement are: " " 
Account Limit :: " (Utilities|String|ToString(Integer) (Variables|Default|GetAccount%20Limit)) " ::  
Withdrawl Fee :: " (.RightS (Utilities|String|Split (Utilities|String|ToString(Float) (Math|Float|Clamp(Float) (Variables|Default|GetFee) 0.0 0.5)) "0.")) "% ::  
Thank you for signing on to " _bankname ". Type !bankhelp in chat for a list of commands!" " 
Your maximum allowed withdrawl for the match is :: " (Utilities|String|ToString(Integer) _maxwithdraw) " ::")))))))

(event EventBeginPlay
  (bind _newparam (CallFunction|GetConfig))
  (if _newparam
    (Actor|DestroyActor)
    (else
      (|CallParentFunction)
      (bind _loadedstringarray (Class|MordhauUtilityLibrary|LoadStringArrayfromFile "PointBank" ".txt"))
      (CallFunction|PreparePointBank _loadedstringarray)
      (bind _asbp_horde_game_mode (Utilities|Casting|CastToBP_HordeGameMode (Game|GetGameMode)))
      (bind _output_get (Variables|Default|SetAs%20BP%20Horde%20Game%20Mode _asbp_horde_game_mode))
      (Development|PrintString (Utilities|GetDisplayName _output_get))
      (EventDispatchers|BindEventtoOnMessageBroadcasted _output_get (EventDispatchers|CreateEvent :!event ExecuteChatCommand))
      (EventDispatchers|BindEventtoOnAfterLogin _output_get (delegate Custom|CustomEvent_1)))))

(event EventTick
  (params (DeltaSeconds :type Float%20%28single-precision%29))
  (bind _as_bp_horde_game_mode (Variables|Default|GetAs%20BP%20Horde%20Game%20Mode))
  (Utilities|IsValid _as_bp_horde_game_mode
    (:Is%20Valid
      (if (Class|GameModeBase|HasMatchEnded _as_bp_horde_game_mode)
        (Utilities|FlowControl|DoOnce false
          (:Completed
            (Class|MordhauUtilityLibrary|SaveStringArraytoFile "PointBank" (Variables|Default|GetPointBank) ".txt")
            (Utilities|BroadcastMacro
              (:Completed
                (CallFunction|Broadcast (Utilities|String|Append (Variables|Default|GetBankName) " has secured all deposited funds for the current match."))))))))))

(fn ConstructionScript
  (|CallParentFunction))

(fn MessageHasCommand
  (params (Message :type String) (Command :type String))
  (LocalVariables|SetMessageX Message)
  (LocalVariables|SetCommandX Command)
  (if (Utilities|String|StartsWith (LocalVariables|GetMessageX) (LocalVariables|GetCommandX))
    (return true (Utilities|String|GetSubstring (LocalVariables|GetMessageX) (Utilities|String|Len (LocalVariables|GetCommandX)) (- (Utilities|String|Len (LocalVariables|GetMessageX)) (Utilities|String|Len (LocalVariables|GetCommandX)))))
    (else
      (return false ""))))

(fn GetPlayer
  (params (Player :type String))
  (bind _asbp_mordhau_game_state (Utilities|Casting|CastToBP_MordhauGameState (Game|GetGameState)))
  (for _array_element (Variables|/Script/Engine.GameStateBase|GetPlayerArray _asbp_mordhau_game_state)
    (if (Utilities|String|Contains (PlayerState|GetPlayerName _array_element) Player)
      (return _array_element true)))
  (return 0 false))

(fn ParseMessage
  (params (Message :type String))
  (bind _output_get (LocalVariables|SetTemp Message))
  (return "invalid" (Math|Conversions|ToInteger(Byte) _output_get) 0))

(fn PrepareEntry
  (params (Controller :type BP%20Horde%20Player%20Controller%20Object%20Reference))
  (bind _pointbank (Variables|Default|GetPointBank))
  (bind _output_get (LocalVariables|SetNewLocalVar_3 (Class|MordhauPlayerController|GetPlayFabID Controller)))
  (if (Utilities|Enum|Equal(Enum) _output_get "")
    (return false -1)
    (else
      (for (_array_element _array_index) _pointbank
        (if (Utilities|String|StartsWith _array_element _output_get)
          (return true _array_index)))
      (bind _returnvalue (Utilities|Array|AddUnique _pointbank (Utilities|String|Append _output_get "=0" "," (Utilities|String|ToString(Integer) (Variables|Default|GetMaxWithdraw)))))
      (return false _returnvalue))))

(fn GetEntryBalance
  (params (Entry :type Integer))
  (bind _output_get (LocalVariables|SetNewLocalVar_0 (Utilities|Array|Get(acopy) (Variables|Default|GetPointBank) Entry)))
  (return (Math|Conversions|ToInteger(Byte) (.LeftS (Utilities|String|Split (.RightS (Utilities|String|Split _output_get "=")) ",")))))

(fn SetEntryBalance
  (params (Entry :type Integer) (Amount :type Integer))
  (bind _output_get (LocalVariables|SetNewLocalVar_1 (Utilities|Array|Get(acopy) (Variables|Default|GetPointBank) Entry)))
  (Utilities|Array|SetArrayElem (Variables|Default|GetPointBank) Entry (Utilities|String|Append (.LeftS (Utilities|String|Split _output_get "= ")) "= " (Utilities|String|ToString(Integer) Amount) "," (Utilities|String|ToString(Integer) (CallFunction|GetAmountLeft Entry))))
  (Variables|Default|SetPointBank (Variables|Default|GetPointBank))
  (Development|PrintString (Utilities|String|Append (.LeftS (Utilities|String|Split _output_get "= ")) "= " (Utilities|String|ToString(Integer) Amount) "," (Utilities|String|ToString(Integer) (CallFunction|GetAmountLeft Entry)))))

(fn IsEntryOverLimit
  (params (Entry :type Integer)))

(fn NotifyDisabled
  (if (Variables|Default|GetIsDisabled)
    (return true)
    (else
      (return false))))

(fn IsSuperAdmin
  (params (Actor :type Actor%20Object%20Reference))
  (bind _asbp_horde_player_controller (Utilities|Casting|CastToBP_HordePlayerController Actor))
  (if (and (Class|MordhauPlayerController|IsAdmin _asbp_horde_player_controller) (Utilities|Array|ContainsItem (Variables|Default|GetSuperAdmins) (Class|MordhauPlayerController|GetPlayFabID _asbp_horde_player_controller)))
    (return true)
    (else
      (return false))))

(fn Broadcast
  (params (Message :type String))
  (Development|PrintString Message)
  (Class|MordhauGameMode|Broadcast (Variables|Default|GetAs%20BP%20Horde%20Game%20Mode) 0 Message "ServerSay"))

(fn GetConfig
  (bind (_arraysize _returnvalue) (Class|MordhauUtilityLibrary|GetCustomConfigVarArray "ServerSideCmd" "SuperAdmin"))
  (bind (_arraysize_2 _returnvalue_2) (Class|MordhauUtilityLibrary|GetCustomConfigVarArray "HordeStuff2" "DisableOnMap"))
  (bind (_isvalid _returnvalue_3) (Class|MordhauUtilityLibrary|GetCustomConfigVarFloat "Hordestuff2" "BankFee"))
  (bind (_isvalid_2 _returnvalue_4) (Class|MordhauUtilityLibrary|GetCustomConfigVarInt "Hordestuff2" "BankMaxWithdraw"))
  (bind (_isvalid_3 _returnvalue_5) (Class|MordhauUtilityLibrary|GetCustomConfigVarInt "Hordestuff2" "BankAccountLimit"))
  (bind (_isvalid_4 _returnvalue_6) (Class|MordhauUtilityLibrary|GetCustomConfigVarString "Hordestuff2" "BankName"))
  (Utilities|FlowControl|Sequence
    (:then_0
      (Utilities|Casting|CastToBP_HordeGameMode (Game|GetGameMode)
        (:then
          (if (> _arraysize_2 0)
            (Variables|Default|SetArray _returnvalue_2)
            (bind _returnvalue_7 (Game|GetCurrentLevelName false))
            (for _array_element (Variables|Default|GetArray)
              (if (Utilities|Enum|Equal(Enum) _returnvalue_7 _array_element)
                (return true)))))
        (:CastFailed
          (return true))))
    (:then_1
      (if _isvalid
        (Variables|Default|SetFee _returnvalue_3)
        (else
          (Variables|Default|SetFee 0.03))))
    (:then_2
      (if _isvalid_3
        (Variables|Default|SetAccount%20Limit _returnvalue_5)
        (else
          (Variables|Default|SetAccount%20Limit 10000))))
    (:then_3
      (if _isvalid_2
        (Variables|Default|SetMaxWithdraw _returnvalue_4)
        (else
          (Variables|Default|SetMaxWithdraw 8000))))
    (:then_4
      (if _isvalid_4
        (Variables|Default|SetBankName _returnvalue_6)
        (else
          (Variables|Default|SetBankName "MORDHAU Financial"))))
    (:then_5
      (if (> _arraysize 0)
        (for _array_element_2 _returnvalue
          (Utilities|Array|AddUnique (Variables|Default|GetSuperAdmins) _array_element_2))
        (Variables|Default|SetSuperAdmins (Variables|Default|GetSuperAdmins))))
    (:then_6
      (return false))))

(fn GetAmountLeft
  (params (Entry :type Integer))
  (bind _output_get (LocalVariables|SetNewLocalVar_0 (Utilities|Array|Get(acopy) (Variables|Default|GetPointBank) Entry)))
  (return (Math|Conversions|ToInteger(Byte) (.RightS (Utilities|String|Split _output_get ",")))))

(fn SetAmountLeft
  (params (Entry :type Integer) (Amount :type Integer))
  (bind _pointbank (Variables|Default|GetPointBank))
  (bind _output_get (LocalVariables|SetNewLocalVar_0 (Utilities|Array|Get(acopy) _pointbank Entry)))
  (Utilities|Array|SetArrayElem _pointbank Entry (Utilities|String|Append (.LeftS (Utilities|String|Split _output_get ",")) "," (Utilities|String|ToString(Integer) Amount))))

(fn PreparePointBank
  (params (RestockArray :type Array%20of%20Strings))
  (bind _output_get (LocalVariables|SetNewLocalVar_2 RestockArray))
  (for (_array_element _array_index) _output_get
    (Utilities|Array|SetArrayElem _output_get _array_index (Utilities|String|Append (.LeftS (Utilities|String|Split _array_element ",")) "," (Utilities|String|ToString(Integer) (Variables|Default|GetMaxWithdraw)))))
  (Variables|Default|SetPointBank _output_get))

(fn ExecuteChatCommand
  (params (Sender :type Actor%20Object%20Reference) (Msg :type String) (Type :type Name))
  (bind _asbp_horde_player_controller (Utilities|Casting|CastToBP_HordePlayerController Sender))
  (LocalVariables|SetNewLocalVar_4 _asbp_horde_player_controller)
  (LocalVariables|SetNewLocalVar_5 Msg)
  (if (.ReturnValue (CallFunction|GetEntry _asbp_horde_player_controller))
    (LocalVariables|SetNewLocalVar_6 (.Array%20Index (CallFunction|GetEntry _asbp_horde_player_controller)))
    (for _array_element (LocalVariables|GetNewLocalVar_0)
      (if (.ReturnValue (CallFunction|MessageHasCommand (LocalVariables|GetNewLocalVar_5) _array_element))
        (bind _isdisabled (CallFunction|NotifyDisabled))
        (if _isdisabled
          (CallFunction|Broadcast (Utilities|String|Append "Sorry, " (Variables|Default|GetBankName) " is closed for the remainder of the match."))
          (else
            (CallFunction|EventChatCommand (Variables|Default|GetAs%20BP%20Horde%20Player%20Controller) _array_element (Variables|Default|GetNewVar_0) (.ReturnValue1 (CallFunction|MessageHasCommand (LocalVariables|GetNewLocalVar_5) _array_element)))))))))

(fn GetEntry
  (params (Controller :type BP%20Horde%20Player%20Controller%20Object%20Reference))
  (bind _output_get (LocalVariables|SetNewLocalVar_3 (Class|MordhauPlayerController|GetPlayFabID Controller)))
  (if (Utilities|Enum|Equal(Enum) _output_get "")
    _
    (else
      (for (_array_element _array_index) (Variables|Default|GetPointBank)
        (if (Utilities|String|StartsWith _array_element _output_get)
          (return true _array_index)))))
  (return false -1))