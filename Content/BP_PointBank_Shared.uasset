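; Server-side actor for Mordhau Horde that runs a shared coin bank, persistent across matches, through chat commands.
; Game mode message and login events drive deposits, fee-charged withdrawals, help and greetings, all announced by delayed server broadcasts.
; Config sets fee, limits and disabled maps; text files store the balance and a PlayFab ID player list.
; Coin cheats from non-super admins disable banking for the rest of the match.
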(event Custom|CustomEvent_0
  (params (Sender :type Actor%20Object%20Reference) (Msg :type String) (Type :type Name))
  (bind _amount (CallFunction|GetCurrentBankBalance))
  (bind (_returnvalue _returnvalue1) (CallFunction|MessageHasCommand Msg "!sdeposit"))
  (bind (_returnvalue_2 _returnvalue1_2) (CallFunction|MessageHasCommand Msg "!swithdraw"))
  (bind _maxwdraw (Variables|Default|GetMaxWdraw))
  (bind _bankname (Variables|Default|GetBankName))
  (bind _account_limit (Variables|Default|GetAccount%20Limit))
  (bind _bankname_2 (Variables|Default|GetBankName))
  (bind _bankname_3 (Variables|Default|GetBankName))
  (bind _bankname_4 (Variables|Default|GetBankName))
  (bind _bankname_5 (Variables|Default|GetBankName))
  (bind _returnvalue_3 (Math|Conversions|ToInteger(Byte) _returnvalue1_2))
  (if (not (Variables|Default|GetPreventRec))
    (Development|PrintString "OnMessageBroadcasted_Event")
    (bind _asbp_horde_player_controller (Utilities|Casting|CastToBP_HordePlayerController Sender))
    (Variables|Default|SetPreventRec true)
    (Variables|Default|SetNewVar_0 0)
    (Utilities|FlowControl|Sequence
      (:then_0
        (if (not (CallFunction|IsSuperAdmin _asbp_horde_player_controller))
          (if (Class|MordhauPlayerController|IsAdmin _asbp_horde_player_controller)
            (if (or (.ReturnValue (CallFunction|MessageHasCommand Msg ".coinsall")) (.ReturnValue (CallFunction|MessageHasCommand Msg ".coins")))
              (Variables|Default|SetIsDisabled true)
              (Utilities|BroadcastMacro
                (:Completed
                  (CallFunction|Broadcast (Utilities|String|Append _bankname_5 " has detected Admin Stimulus, to prevent Inflation, " _bankname_5 " has shut down for the remainder of the match. No deposits or withdrawl's can be made."))))))))
      (:then_1
        (if _returnvalue
          (bind _output_get (Variables|Default|SetNewVar_0 (Math|Conversions|ToInteger(Byte) _returnvalue1)))
          (if (> _output_get 0)
            (bind _isdisabled (CallFunction|NotifyDisabled))
            (if (not _isdisabled)
              (bind _asbp_horde_player_state (Utilities|Casting|CastToBP_HordePlayerState (Variables|/Script/Engine.Controller|GetPlayerState _asbp_horde_player_controller)))
              (if (>= (Variables|/Game/Mordhau/Blueprints/GameModes/Horde/BP_HordePlayerState.BP_HordePlayerState_C|GetCoins _asbp_horde_player_state) _output_get)
                (Utilities|BroadcastMacro
                  (:Completed
                    (CallFunction|Broadcast (Utilities|String|Append (PlayerState|GetPlayerName _asbp_horde_player_state) " has attempted to deposit :: " (Utilities|String|ToString(Integer) _output_get) " :: Coins to " _bankname_3))
                    (if (> (+ _output_get (CallFunction|GetCurrentBankBalance)) _account_limit)
                      (Utilities|BroadcastMacro
                        (:Completed
                          (CallFunction|Broadcast (Utilities|String|Append _bankname_2 " Teller: Sorry " (PlayerState|GetPlayerName _asbp_horde_player_state) ", this would put you over the max allowed amount for the account. Your Max allowed amount is currently :: " (Utilities|String|ToString(Integer) _account_limit) " ::"))))
                      (else
                        (Utilities|BroadcastMacro
                          (:Completed
                            (CallFunction|Broadcast (Utilities|String|Append _bankname_2 " Teller: Server account balance has been updated, your new current amount is :: " (Utilities|String|ToString(Integer) (+ _output_get (CallFunction|GetCurrentBankBalance))) " :: Thank you for being a valued customer of " _bankname_2 (Utilities|Select :Index (Math|Random|RandomIntegerinRange 0 5) :Option%200 (Utilities|String|Append ". Slay them all " (PlayerState|GetPlayerName _asbp_horde_player_state) "!") :Option%201 ". Enjoy the Match!" :Option%202 ". I am humbled by your skills, sir!" :Option%203 ". Your form, and execution, are exquisite!" :Option%204 ". It is an honor to meet such a fine combatant!" :Option%205 ". You have the heart of a lion!")))
                            (CallFunction|SetCurrentBankBalance (+ _output_get (CallFunction|GetCurrentBankBalance)))
                            (Variables|/Game/Mordhau/Blueprints/GameModes/Horde/BP_HordePlayerState.BP_HordePlayerState_C|SetCoins _asbp_horde_player_state (- (Variables|/Game/Mordhau/Blueprints/GameModes/Horde/BP_HordePlayerState.BP_HordePlayerState_C|GetCoins _asbp_horde_player_state) _output_get))))))))
                (else
                  (Utilities|BroadcastMacro
                    (:Completed
                      (CallFunction|Broadcast (Utilities|String|Append _bankname_3 " Teller: " (PlayerState|GetPlayerName _asbp_horde_player_state) ", you do not have enough coins to make this Deposit."))))))))
          (elif _returnvalue_2
            (bind _isdisabled_2 (CallFunction|NotifyDisabled))
            (if (not _isdisabled_2)
              (if (> _returnvalue_3 _maxwdraw)
                (Utilities|BroadcastMacro
                  (:Completed
                    (CallFunction|Broadcast (Utilities|String|Append (Variables|Default|GetBankName) " Teller: Sorry, you cannot withdraw more than :: " (Utilities|String|ToString(Integer) _maxwdraw) " :: At a time per bank rules."))))
                (else
                  (bind _output_get_2 (Variables|Default|SetNewVar_0 _returnvalue_3))
                  (if (and (> _output_get_2 0) (not (> _output_get_2 (Variables|Default|GetMaxWithdraw))))
                    (bind _asbp_horde_player_state_2 (Utilities|Casting|CastToBP_HordePlayerState (Variables|/Script/Engine.Controller|GetPlayerState _asbp_horde_player_controller)))
                    (Utilities|BroadcastMacro
                      (:Completed
                        (CallFunction|Broadcast (Utilities|String|Append (PlayerState|GetPlayerName _asbp_horde_player_state_2) " has attempted to withdraw :: " (Utilities|String|ToString(Integer) _output_get_2) " :: Coins from " _bankname ". With a Fee of :: " (Utilities|String|ToString(Integer) (Math|Float|Truncate (* _output_get_2 (Variables|Default|GetFee)))) " ::"))
                        (if (>= _amount (+ _output_get_2 (Math|Float|Truncate (* _output_get_2 (Variables|Default|GetFee)))))
                          (Utilities|BroadcastMacro
                            (:Completed
                              (bind _output_get_3 (Variables|Default|SetMaxWithdraw (- (Variables|Default|GetMaxWithdraw) _output_get_2)))
                              (CallFunction|Broadcast (Utilities|String|Append _bankname_4 "Teller: Your withdrawl is accepted. Account balance has been updated, new current balance is :: " (Utilities|String|ToString(Integer) (- _amount (+ _output_get_2 (Math|Float|Truncate (* _output_get_2 (Variables|Default|GetFee)))))) " :: Thank you for being a valued customer of " _bankname_4 (Utilities|Select :Index (Math|Random|RandomIntegerinRange 0 5) :Option%200 (Utilities|String|Append ". Slay them all " (PlayerState|GetPlayerName _asbp_horde_player_state) "!") :Option%201 ". Enjoy the Match!" :Option%202 ". I am humbled by your skills, sir!" :Option%203 ". Your form, and execution, are exquisite!" :Option%204 ". It is an honor to meet such a fine combatant!" :Option%205 ". You have the heart of a lion!") " 
There is currently :: " (Utilities|String|ToString(Integer) _output_get_3) " :: Left in the bank for the current match."))
                              (CallFunction|SetCurrentBankBalance (- _amount (+ _output_get_2 (Math|Float|Truncate (* _output_get_2 (Variables|Default|GetFee))))))
                              (Variables|/Game/Mordhau/Blueprints/GameModes/Horde/BP_HordePlayerState.BP_HordePlayerState_C|SetCoins _asbp_horde_player_state_2 (+ (Variables|/Game/Mordhau/Blueprints/GameModes/Horde/BP_HordePlayerState.BP_HordePlayerState_C|GetCoins _asbp_horde_player_state_2) _output_get_2))))
                          (else
                            (Utilities|BroadcastMacro
                              (:Completed
                                (CallFunction|Broadcast (Utilities|String|Append _bankname " Teller: Sorry " (PlayerState|GetPlayerName _asbp_horde_player_state_2) ", There is not enough coins in the bank to make this Transaction. "))))))))
                    (else
                      (Utilities|BroadcastMacro
                        (:Completed
                          (CallFunction|Broadcast (Utilities|String|Append (Variables|Default|GetBankName) " Teller: Sorry, there is not enough available funds left in the bank to make this transaction.")))))))))
            (elif (.ReturnValue (CallFunction|MessageHasCommand Msg "!sbankhelp"))
              (Variables|Default|SetNewVar_1 "")
              (bind _isdisabled_3 (CallFunction|NotifyDisabled))
              (bind _remainingwithdrawl (CallFunction|PrepareEntry _asbp_horde_player_controller))
              (Variables|Default|SetNewVar_1 (Utilities|String|Append "Help Menu 
" "!sdeposit amount       
 // Deposits the specified amount, assuming you have it. 
!swithdraw amount  
// Will withdraw from bank account if you have the funds/the bank has the funds. 
 
Current Account Balance :: " (Utilities|String|ToString(Integer) (CallFunction|GetCurrentBankBalance)) " :: 
Bank Status :: " (Utilities|String|SelectString "DISABLED" "ENABLED" _isdisabled_3) " :: 
Remaining server bank funds for the match :: " (Utilities|String|ToString(Integer) (Variables|Default|GetMaxWithdraw)) " ::" "Your current available withdrawl amount remaining :: " (Utilities|String|ToString(Integer) _remainingwithdrawl) " ::"))
              (Utilities|BroadcastMacro
                (:Completed
                  (CallFunction|Broadcast (Utilities|String|Append "Help Menu 
" "!sdeposit amount       
 // Deposits the specified amount, assuming you have it. 
!swithdraw amount  
// Will withdraw from bank account if you have the funds/the bank has the funds. 
 
Current Account Balance :: " (Utilities|String|ToString(Integer) (CallFunction|GetCurrentBankBalance)) " :: 
Bank Status :: " (Utilities|String|SelectString "DISABLED" "ENABLED" _isdisabled_3) " :: 
Remaining server bank funds for the match :: " (Utilities|String|ToString(Integer) (Variables|Default|GetMaxWithdraw)) " ::" "Your current available withdrawl amount remaining :: " (Utilities|String|ToString(Integer) _remainingwithdrawl) " ::"))))))))
      (:then_2
        (Variables|Default|SetPreventRec false)))))

(event Custom|CustomEvent_1
  (params (NewPlayer :type Player%20Controller%20Object%20Reference))
  (bind _bankname (Variables|Default|GetBankName))
  (bind _maxwithdraw (Variables|Default|GetMaxWithdraw))
  (bind _isdisabled (Variables|Default|GetIsDisabled))
  (bind _returnvalue (Utilities|String|SelectString "DISABLED" "ENABLED" _isdisabled))
  (Utilities|FlowControl|Delay 1.0)
  (Development|PrintString "OnAfterLogin_Event")
  (bind _asbp_horde_player_controller (Utilities|Casting|CastToBP_HordePlayerController NewPlayer))
  (bind (_returnvalue_2 _remainingwithdrawl) (CallFunction|PrepareEntry _asbp_horde_player_controller))
  (if _returnvalue_2
    (Utilities|BroadcastMacro
      (:Completed
        (CallFunction|Broadcast (Utilities|String|Append _bankname " is " _returnvalue ". " (PlayerState|GetPlayerName (Variables|/Script/Engine.Controller|GetPlayerState _asbp_horde_player_controller)) ", your account has been found in our database, the current balance of our shared account is :: " (Utilities|String|ToString(Integer) (CallFunction|GetCurrentBankBalance)) " :: Type !sbankhelp in chat for a list of commands!" " 
The current remaining bank withdrawl balance for the match is :: " (Utilities|String|ToString(Integer) _maxwithdraw) " :: 
Your current available withdrawl amount remaining :: " (Utilities|String|ToString(Integer) _remainingwithdrawl) " ::"))))
    (else
      (Utilities|BroadcastMacro
        (:Completed
          (CallFunction|Broadcast (Utilities|String|Append _bankname " is " _returnvalue ". Welcome New Customer! You are currently not signed up for our services, lets change that. The terms of agreement are: " " 
Server Shared Account Limit :: " (Utilities|String|ToString(Integer) (Variables|Default|GetAccount%20Limit)) " ::  
Withdrawl Fee :: " (.RightS (Utilities|String|Split (Utilities|String|ToString(Float) (Math|Float|Clamp(Float) (Variables|Default|GetFee) 0.0 0.5)) "0.")) "% ::  
Thank you for signing on to " _bankname ". Type !sbankhelp in chat for a list of commands!" " 
The current remaining bank withdrawl balance for the match is :: " (Utilities|String|ToString(Integer) _maxwithdraw) " ::" "Your current available withdrawl amount remaining ::  " (Utilities|String|ToString(Integer) (Variables|Default|GetMaxWdraw)) " ::")))))))

(event EventBeginPlay
  (bind _newparam (CallFunction|GetConfig))
  (if _newparam
    (Actor|DestroyActor)
    (else
      (|CallParentFunction)
      (bind _loadedstringarray (Class|MordhauUtilityLibrary|LoadStringArrayfromFile "PointBank_Shared" ".txt"))
      (bind _output_get (Variables|Default|SetPointBank _loadedstringarray))
      (CallFunction|PreparePointBank _output_get)
      (bind _loadedstring (Class|MordhauUtilityLibrary|LoadStringfromFile "PointBank_Shared_Balance" ".txt"))
      (Variables|Default|SetBankBalance (Math|Conversions|ToInteger(Byte) _loadedstring))
      (bind _asbp_horde_game_mode (Utilities|Casting|CastToBP_HordeGameMode (Game|GetGameMode)))
      (bind _output_get_2 (Variables|Default|SetAs%20BP%20Horde%20Game%20Mode _asbp_horde_game_mode))
      (Development|PrintString (Utilities|GetDisplayName _output_get_2))
      (EventDispatchers|BindEventtoOnMessageBroadcasted _output_get_2 (delegate Custom|CustomEvent_0))
      (EventDispatchers|BindEventtoOnAfterLogin _output_get_2 (delegate Custom|CustomEvent_1)))))

(event EventTick
  (params (DeltaSeconds :type Float%20%28single-precision%29))
  (bind _bankbalance (Variables|Default|GetBankBalance))
  (bind _as_bp_horde_game_mode (Variables|Default|GetAs%20BP%20Horde%20Game%20Mode))
  (Utilities|IsValid _as_bp_horde_game_mode
    (:Is%20Valid
      (if (Class|GameModeBase|HasMatchEnded _as_bp_horde_game_mode)
        (Utilities|FlowControl|DoOnce false
          (:Completed
            (Class|MordhauUtilityLibrary|SaveStringArraytoFile "PointBank_Shared" (Variables|Default|GetPointBank) ".txt")
            (Utilities|FlowControl|Sequence
              (:then_0
                (if (not (== _bankbalance (CallFunction|GetCurrentBankBalance)))
                  (CallFunction|SetCurrentBankBalance _bankbalance)))
              (:then_1
                (Utilities|BroadcastMacro
                  (:Completed
                    (CallFunction|Broadcast (Utilities|String|Append (Variables|Default|GetBankName) " has secured all deposited funds for the current match."))))))))))))

(fn ConstructionScript
  (|CallParentFunction))

(fn MessageHasCommand
  (params (Message :type String) (Command :type String))
  (LocalVariables|SetMessageX Message)
  (LocalVariables|SetCommandX Command)
  (if (Utilities|String|StartsWith (LocalVariables|GetMessageX) (LocalVariables|GetCommandX))
    (return true (Utilities|String|GetSubstring (LocalVariables|GetMessageX) (Utilities|String|Len (LocalVariables|GetCommandX)) (- (Utilities|String|Len (LocalVariables|GetMessageX)) (Utilities|String|Len (LocalVariables|GetCommandX)))))
    (else
      (return false ""))))

(fn GetPlayer
  (params (Player :type String))
  (bind _asbp_mordhau_game_state (Utilities|Casting|CastToBP_MordhauGameState (Game|GetGameState)))
  (for _array_element (Variables|/Script/Engine.GameStateBase|GetPlayerArray _asbp_mordhau_game_state)
    (if (Utilities|String|Contains (PlayerState|GetPlayerName _array_element) Player)
      (return _array_element true)))
  (return 0 false))

(fn ParseMessage
  (params (Message :type String))
  (bind _output_get (LocalVariables|SetTemp Message))
  (return "invalid" (Math|Conversions|ToInteger(Byte) _output_get) 0))

(fn PrepareEntry
  (params (Controller :type BP%20Horde%20Player%20Controller%20Object%20Reference))
  (bind _pointbank (Variables|Default|GetPointBank))
  (bind _output_get (LocalVariables|SetNewLocalVar_3 (Class|MordhauPlayerController|GetPlayFabID Controller)))
  (for _array_element _pointbank
    (if (Utilities|String|StartsWith _array_element _output_get)
      (return true (Math|Conversions|ToInteger(Byte) (.RightS (Utilities|String|Split _array_element ","))))))
  (Utilities|Array|AddUnique _pointbank (Utilities|String|Append _output_get "," (Utilities|String|ToString(Integer) (Variables|Default|GetMaxWdraw))))
  (return false 0))

(fn GetCurrentBankBalance
  (bind _loadedstring (Class|MordhauUtilityLibrary|LoadStringfromFile "PointBank_Shared_Balance" ".txt"))
  (bind _output_get (Variables|Default|SetBankBalance (Math|Conversions|ToInteger(Byte) _loadedstring)))
  (return _output_get))

(fn SetCurrentBankBalance
  (params (Amount :type Integer))
  (bind _output_get (Variables|Default|SetBankBalance Amount))
  (Class|MordhauUtilityLibrary|SaveStringtoFile "PointBank_Shared_Balance" (Utilities|String|ToString(Integer) _output_get) ".txt"))

(fn IsEntryOverLimit
  (params (Entry :type Integer)))

(fn NotifyDisabled
  (if (Variables|Default|GetIsDisabled)
    (CallFunction|Broadcast (Utilities|String|Append "Sorry, " (Variables|Default|GetBankName) " is closed for the remainder of the match."))
    (return true)
    (else
      (return false))))

(fn IsSuperAdmin
  (params (Actor :type Actor%20Object%20Reference))
  (bind _asbp_horde_player_controller (Utilities|Casting|CastToBP_HordePlayerController Actor))
  (if (and (Class|MordhauPlayerController|IsAdmin _asbp_horde_player_controller) (Utilities|Array|ContainsItem (Variables|Default|GetSuperAdmins) (Class|MordhauPlayerController|GetPlayFabID _asbp_horde_player_controller)))
    (return true)
    (else
      (return false))))

(fn Broadcast
  (params (Message :type String))
  (Development|PrintString Message)
  (Class|MordhauGameMode|Broadcast (Variables|Default|GetAs%20BP%20Horde%20Game%20Mode) 0 Message "ServerSay"))

(fn GetConfig
  (bind (_arraysize _returnvalue) (Class|MordhauUtilityLibrary|GetCustomConfigVarArray "ServerSideCmd" "SuperAdmin"))
  (bind (_arraysize_2 _returnvalue_2) (Class|MordhauUtilityLibrary|GetCustomConfigVarArray "HordeStuff2" "DisableOnMap"))
  (bind (_isvalid _returnvalue_3) (Class|MordhauUtilityLibrary|GetCustomConfigVarFloat "Hordestuff2" "SBankFee"))
  (bind (_isvalid_2 _returnvalue_4) (Class|MordhauUtilityLibrary|GetCustomConfigVarInt "Hordestuff2" "SBankMaxWithdraw"))
  (bind (_isvalid_3 _returnvalue_5) (Class|MordhauUtilityLibrary|GetCustomConfigVarInt "Hordestuff2" "SBankAccountLimit"))
  (bind (_isvalid_4 _returnvalue_6) (Class|MordhauUtilityLibrary|GetCustomConfigVarString "Hordestuff2" "SBankName"))
  (bind (_isvalid_5 _returnvalue_7) (Class|MordhauUtilityLibrary|GetCustomConfigVarInt "Hordestuff2" "SBankTotalWithdraw"))
  (Utilities|FlowControl|Sequence
    (:then_0
      (Utilities|Casting|CastToBP_HordeGameMode (Game|GetGameMode)
        (:then
          (if (> _arraysize_2 0)
            (Variables|Default|SetArray _returnvalue_2)
            (bind _returnvalue_8 (Game|GetCurrentLevelName false))
            (for _array_element (Variables|Default|GetArray)
              (if (Utilities|Enum|Equal(Enum) _returnvalue_8 _array_element)
                (return true)))))
        (:CastFailed
          (return true))))
    (:then_1
      (if _isvalid
        (Variables|Default|SetFee _returnvalue_3)
        (else
          (Variables|Default|SetFee 0.03))))
    (:then_2
      (if _isvalid_3
        (Variables|Default|SetAccount%20Limit _returnvalue_5)
        (else
          (Variables|Default|SetAccount%20Limit 10000))))
    (:then_3
      (if _isvalid_5
        (Variables|Default|SetMaxWithdraw _returnvalue_7)
        (else
          (Variables|Default|SetMaxWithdraw 8000))))
    (:then_4
      (if _isvalid_4
        (Variables|Default|SetBankName _returnvalue_6)
        (else
          (Variables|Default|SetBankName "MORDHAU Server Financial"))))
    (:then_5
      (if (> _arraysize 0)
        (for _array_element_2 _returnvalue
          (Utilities|Array|AddUnique (Variables|Default|GetSuperAdmins) _array_element_2))
        (Variables|Default|SetSuperAdmins (Variables|Default|GetSuperAdmins))))
    (:then_6
      (if _isvalid_2
        (Variables|Default|SetMaxWdraw _returnvalue_4)
        (else
          (Variables|Default|SetMaxWdraw 2000))))
    (:then_7
      (return false))))

(fn PreparePointBank
  (params (RestockArray :type Array%20of%20Strings))
  (bind _output_get (LocalVariables|SetNewLocalVar_2 RestockArray))
  (for (_array_element _array_index) _output_get
    (Utilities|Array|SetArrayElem _output_get _array_index (Utilities|String|Append (.LeftS (Utilities|String|Split _array_element ",")) "," (Utilities|String|ToString(Integer) (Variables|Default|GetMaxWithdraw)))))
  (Variables|Default|SetPointBank _output_get))